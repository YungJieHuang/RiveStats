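; BP_RiveActor is an actor that shows the Rive "pause_exit_menu" artboard as a full-viewport UI overlay.
; On BeginPlay it waits for the Rive file, instantiates the artboard, and adds a widget that displays the render target to the viewport.
; Each tick resizes the target to the viewport, and the artboard's render callback draws it stretched to fill.
; An inverse draw-transform function maps texture positions to artboard coordinates.
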(event `self.ReceiveBeginPlay`
  (bind _rive_file (`self.Rive File`))
  (`RiveFileWhenReadyAsync.RiveFileWhenReadyAsync` _rive_file
    (:`Ready`
      (bind _returnvalue (`RiveActorComponent.InstantiateArtboard` (`self.RiveActor`) _rive_file "pause_exit_menu" ""))
      (bind _output_get (set `self.Artboard` _returnvalue))
      (set `RiveArtboard.OnArtboardTick_Render` (delegate `Align`) _output_get)
      (set `RiveArtboard.OnGetLocalCoordinate` (`|CreateDelegate` :!event `TrasferTransfrom`) (`self.Artboard`))
      (bind _returnvalue_2 (`|CreateWidget` "/Script/Rive.RiveImageUserWidget"))
      (bind _output_get_2 (set `self.Widget` _returnvalue_2))
      (`RiveImageUserWidget.Setup` _output_get_2 (`RiveActorComponent.RenderTarget` (`self.RiveActor`)) (`|MakeArray` (`self.Artboard`)))
      (`UserWidget.AddToViewport` (`self.Widget`) 0))))

(event `Align`
  (params (DeltaTime :type "Float (single-precision)") (Artboard :type "RiveArtboard Object Reference"))
  (`RiveArtboard.Align` Artboard (`KismetMathLibrary.MakeBox2D` (0.0 0.0) (`KismetMathLibrary.Conv_IntPointToVector2D` (`RiveTexture.Size` (`RiveActorComponent.RenderTarget` (`self.RiveActor`))))) "Fill" "TopLeft")
  (`RiveArtboard.Draw` Artboard))

(event `self.ReceiveTick`
  (params (DeltaSeconds :type "Float (single-precision)"))
  (bind (_x _y) (`KismetMathLibrary.BreakVector2D` (`WidgetLayoutLibrary.GetViewportSize`)))
  (`RiveActorComponent.ResizeRenderTarget` (`self.RiveActor`) (`KismetMathLibrary.FTrunc` _x) (`KismetMathLibrary.FTrunc` _y)))

(fn `TrasferTransfrom`
  (params (Artboard :type "RiveArtboard Object Reference") (TexturePosition :type "Vector2f Structure (by ref)"))
  (returns (ReturnValue :type "Vector2f Structure"))
  (return (`KismetMathLibrary.Conv_VectorToVector2D` (`KismetMathLibrary.Matrix_InverseTransformPosition` (`RiveArtboard.GetLastDrawTransformMatrix` Artboard) (`KismetMathLibrary.Conv_Vector2DToVector` TexturePosition)))))

(fn `UserConstructionScript`)